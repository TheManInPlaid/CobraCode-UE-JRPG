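; Turn-based battle manager that spawns warrior party and slime enemies, possesses itself as the swaying camera view, and cycles turns.
; Turn order is party then enemies, refilled when empty; the first entry is always active.
; Party members slide to an active spot and back via timelines, while enemies just wait.
; Combat is placeholder: a fixed delay after the first turn starts reopens the field level named by the game instance.
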(event `self.ReceiveBeginPlay`
  (`TimelineComponent.SetPlayRate` (`self.AnimMoveToActiveLocation`) 2.0) ; TODO: Remove magic number for playrate
  (`TimelineComponent.SetPlayRate` (`self.AnimMoveBackFromActiveLocation`) 2.0)
  (`self.StartBattle`))

(event `StartCameraSway`
  (bind (_relativerotation_roll _relativerotation_pitch) (`KismetMathLibrary.BreakRotator` (`SceneComponent.RelativeRotation` (`self.Camera`))))
  (`TimelineComponent.SetPlayRate` (`self.AnimCameraSway`) (`self.CameraSwayRate`))
  (bind (_direction _yawrotation) (`Timeline|AnimCameraSway` :!via `PlayFromStart`)
    (:`Update`
      (`SceneComponent.K2_SetRelativeRotation` (`self.Camera`) (`KismetMathLibrary.MakeRotator` _relativerotation_roll _relativerotation_pitch (* _yawrotation (`self.CameraSwayDistance`))) false false))))

(event `StartBattle`
  (for _array_element (`self.EnemyBattleLocations`)
    (bind _returnvalue (`|SpawnActorFromClass` "/Game/Blueprints/Battle/BattleChars/Enemies/Slime/BP_BattleChar_Enemy_Slime.BP_BattleChar_Enemy_Slime_C" (`KismetMathLibrary.MakeTransform` (+ _array_element (`self.K2_GetActorLocation`) (`self.SpawnHeightOffset`))) "AlwaysSpawn" "MultiplyWithRoot" null null))
    (`KismetArrayLibrary.Array_AddUnique` (`self.EnemyParty`) _returnvalue))
  (for _array_element_2 (`self.PartyBattleLocations`)
    (bind _returnvalue_2 (`|SpawnActorFromClass` "/Game/Blueprints/Battle/BattleChars/Party/Warrior/BP_BattleChar_Party_Warrior.BP_BattleChar_Party_Warrior_C" (`KismetMathLibrary.MakeTransform` (+ _array_element_2 (`self.K2_GetActorLocation`) (`self.SpawnHeightOffset`)) (`self.PartyBattleRotation`)) "AlwaysSpawn" "MultiplyWithRoot" null null))
    (`KismetArrayLibrary.Array_AddUnique` (`self.PlayerParty`) _returnvalue_2))
  (`self.StartCameraSway`)
  (`self.DecideTurnOrder`)
  (`self.SelectActiveCharacter`)
  (`Controller.Possess` (`GameplayStatics.GetPlayerController` 0) self)
  (`self.StartTurn`)
  (`KismetSystemLibrary.Delay` 5.0)
  (`self.ConcludeBattle`))

(event `ConcludeBattle`
  (bind _playerfieldposition (message `/Game/Definitions/Interfaces/BPI_InstanceStorage.I_GetPlayerFieldPosition` (`GameplayStatics.GetGameInstance`)))
  (`GameplayStatics.OpenLevel` (`KismetStringLibrary.Conv_StringToName` (`.FieldLevelName_5_CE03CBE149E0619E33E6C38E0484250A` (break `/Game/Definitions/Structs/S_FieldPosition` _playerfieldposition)))))

(event `StartTurn`
  (`KismetSystemLibrary.PrintString` (`KismetStringLibrary.Concat_StrStr` (`KismetSystemLibrary.GetDisplayName` (`self.ActiveBattleChar`)) " is active"))
  (if (`/Game/Blueprints/Battle/BattleChars/BP_BattleChar_BASE.IsPartyMember` (`self.ActiveBattleChar`))
    (`self.MoveToActiveLocation`)
    (else
      (`KismetSystemLibrary.Delay` 2.0)
      (`self.ConcludeTurn`))))

(event `MoveToActiveLocation`
  ;[0.15 0.1487 0 0.5] Move to Active Location
  (bind (_direction _alpha) (`Timeline|AnimMoveToActiveLocation` :!via `PlayFromStart`)
    (:`Update`
      (`self.K2_SetActorLocation` (`self.ActiveBattleChar`) (`KismetMathLibrary.VLerp` (`/Game/Blueprints/Battle/BattleChars/BP_BattleChar_BASE.BattleSpawnLocation` (`self.ActiveBattleChar`)) (`self.AdjustedActiveLocation`) _alpha) false false))
    (:`Finished`
      (`KismetSystemLibrary.Delay` 2.0)
      (`self.MoveBackFromActiveLocation`))))

(event `MoveBackFromActiveLocation`
  ;[0.15 0.1487 0 0.5] Move Back From Active Location
  (bind (_direction _alpha) (`Timeline|AnimMoveBackFromActiveLocation` :!via `PlayFromStart`)
    (:`Update`
      (`self.K2_SetActorLocation` (`self.ActiveBattleChar`) (`KismetMathLibrary.VLerp` (`self.AdjustedActiveLocation`) (`/Game/Blueprints/Battle/BattleChars/BP_BattleChar_BASE.BattleSpawnLocation` (`self.ActiveBattleChar`)) _alpha) false false))
    (:`Finished`
      (`KismetSystemLibrary.Delay` 1.0)
      (`self.ConcludeTurn`))))

(event `ConcludeTurn`
  (`KismetArrayLibrary.Array_RemoveItem` (`self.TurnOrder`) (`self.ActiveBattleChar`))
  (if (`KismetArrayLibrary.Array_IsEmpty` (`self.TurnOrder`))
    (`self.DecideTurnOrder`)
    (`self.SelectActiveCharacter`)
    (`self.StartTurn`)
    (else
      (`self.SelectActiveCharacter`)
      (`self.StartTurn`))))

(fn `DecideTurnOrder`
  (`KismetArrayLibrary.Array_Clear` (`self.TurnOrder`))
  (`KismetArrayLibrary.Array_Append` (`self.TurnOrder`) (`self.PlayerParty`))
  (`KismetArrayLibrary.Array_Append` (`self.TurnOrder`) (`self.EnemyParty`)))

(fn `SelectActiveCharacter`
  (set `self.ActiveBattleChar` (`|GetArrayItem` (`self.TurnOrder`))))

(fn `UserConstructionScript`)